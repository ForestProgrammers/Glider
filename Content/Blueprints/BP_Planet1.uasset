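; Planet actor that orbits its parent Sun on a spring arm, leaving a debug-point trail.
; Tick advances an angle by Period and feeds CalculateElipseParams results into arm length and yaw for an elliptical, focus-centred orbit.
; That function shows only unconnected law-of-cosines math; an older offset-rotation orbit also never runs.
; Construction creates a dynamic planet material with spin and cloud speeds; Tick keeps its light direction aimed at the Sun.
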(event EventTick
  (params (DeltaSeconds :type Float%20%28single-precision%29))
  (bind _returnvalue (Math|Float|MakeLiteralFloat 1.2))
  (bind (_distancetofocus _aglerotationaroundfocus) (Utilities|CalculateElipseParams _returnvalue))
  (Variables|Default|SetcurrentAgle (select (> (+ (Variables|Default|GetcurrentAgle) (* (/ DeltaSeconds (Variables|Default|GetPeriod)) 3.6e+02)) 3.6e+02) (- (+ (Variables|Default|GetcurrentAgle) (* (/ DeltaSeconds (Variables|Default|GetPeriod)) 3.6e+02)) 3.6e+02) (+ (Variables|Default|GetcurrentAgle) (* (/ DeltaSeconds (Variables|Default|GetPeriod)) 3.6e+02))))
  (Variables|/Script/Engine.SpringArmComponent|SetTargetArmLength (Variables|Default|GetSpringArm) _distancetofocus)
  (Rendering|Debug|DrawDebugPoint (Transformation|GetWorldLocation (Variables|Default|GetStaticMesh)) 1.0 "(R=1.000000,G=0.000000,B=0.111397,A=1.000000)" (* (Variables|Default|GetPeriod) 2.0))
  (Transformation|SetRelativeRotation (Variables|Default|GetSpringArm) (Math|Rotator|MakeRotator 0.0 0.0 _aglerotationaroundfocus) false false)
  (Utilities|IsValid (Variables|Default|GetSun)
    (:Is%20Valid
      ;[1 1 1] set light direction
      (Rendering|Material|SetVectorParameterValue (Variables|Default|GetMaterialInstance) "Light Direction" (Math|Conversions|ToLinearColor(Vector) (Math|Vector|GetForwardVector (Math|Rotator|FindLookatRotation (Transformation|GetActorLocation) (Transformation|GetActorLocation (Variables|Default|GetSun))))) :!class /Script/Engine.MaterialInstanceDynamic))))

(event EventBeginPlay
  (Variables|Default|SetSun (Actor|GetParentActor)))

(fn ConstructionScript
  (bind _sun (Variables|Default|GetSun))
  (Utilities|FlowControl|Sequence
    (:then_0
      (bind _returnvalue (Rendering|Material|CreateDynamicMaterialInstance (Variables|Default|GetStaticMesh) 0 "/Game/Materials/M_PlanetShader_Inst.M_PlanetShader_Inst" :!class /Script/Engine.PrimitiveComponent))
      (Variables|Default|SetMaterialInstance _returnvalue)
      (Rendering|Material|SetVectorParameterValue _returnvalue "Rotation Speed" (Math|Conversions|ToLinearColor(Vector) (Variables|Default|GetRotationSpeed)) :!class /Script/Engine.MaterialInstanceDynamic)
      (Rendering|Material|SetVectorParameterValue _returnvalue "Clouds Speed" (Math|Conversions|ToLinearColor(Vector) (Variables|Default|GetCloudsSpeed)) :!class /Script/Engine.MaterialInstanceDynamic)
      (Utilities|IsValid _sun
        (:Is%20Valid
          (Rendering|Material|SetVectorParameterValue _returnvalue "Light Direction" (Math|Conversions|ToLinearColor(Vector) (Math|Vector|GetForwardVector (Math|Rotator|FindLookatRotation (Transformation|GetActorLocation) (Transformation|GetActorLocation _sun)))) :!class /Script/Engine.MaterialInstanceDynamic))))
    (:then_1
      (Variables|/Script/Engine.SpringArmComponent|SetTargetArmLength (Variables|Default|GetSpringArm) (Variables|Default|GetorbitSize)))))