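; Short-lived splash actor that feeds a location and power into the PostPrc material parameter collection, apparently for a post-process effect.
; Each splash claims one of ten numbered time, power and point slots in round-robin order, using a counter stored in the collection itself.
; A timeline animates that slot's time parameter, then resets it to zero and destroys the actor after a short delay.
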(event Custom|splash
  (params (location :type Vector) (power :type Float%20%28single-precision%29))
  (bind (_x _y _z) (Math|Vector|BreakVector location))
  (bind _returnvalue (Rendering|Material|GetScalarParameterValue "/Game/SciFiGlitchPostPro/PostProcess/Material/postPrc.postPrc" "id" :!class /Script/Engine.KismetMaterialLibrary))
  (if (> (+ _returnvalue 1.0) 1e+01)
    (Rendering|Material|SetScalarParameterValue "/Game/SciFiGlitchPostPro/PostProcess/Material/postPrc.postPrc" "id" 1.0 :!class /Script/Engine.KismetMaterialLibrary)
    (Variables|Default|Setid 1)
    (else
      (Rendering|Material|SetScalarParameterValue "/Game/SciFiGlitchPostPro/PostProcess/Material/postPrc.postPrc" "id" (+ _returnvalue 1.0) :!class /Script/Engine.KismetMaterialLibrary)
      (Variables|Default|Setid (Math|Float|Truncate (+ _returnvalue 1.0)))))
  (Rendering|Material|SetScalarParameterValue "/Game/SciFiGlitchPostPro/PostProcess/Material/postPrc.postPrc" (Utilities|String|StringToName (Utilities|String|Append "time" (Utilities|String|ToString(Integer) (Variables|Default|Getid)))) 0.0 :!class /Script/Engine.KismetMaterialLibrary)
  (Rendering|Material|SetScalarParameterValue "/Game/SciFiGlitchPostPro/PostProcess/Material/postPrc.postPrc" (Utilities|String|StringToName (Utilities|String|Append "power" (Utilities|String|ToString(Integer) (Variables|Default|Getid)))) power :!class /Script/Engine.KismetMaterialLibrary)
  (Rendering|Material|SetVectorParameterValue "/Game/SciFiGlitchPostPro/PostProcess/Material/postPrc.postPrc" (Utilities|String|StringToName (Utilities|String|Append "point" (Utilities|String|ToString(Integer) (Variables|Default|Getid)))) (Utilities|Struct|MakeLinearColor _x _y _z 0.0) :!class /Script/Engine.KismetMaterialLibrary)
  (bind _newtrack_0 (Timeline|Timeline_0 PlayFromStart)
    (:Update
      (Rendering|Material|SetScalarParameterValue "/Game/SciFiGlitchPostPro/PostProcess/Material/postPrc.postPrc" (Utilities|String|StringToName (Utilities|String|Append "time" (Utilities|String|ToString(Integer) (Variables|Default|Getid)))) _newtrack_0 :!class /Script/Engine.KismetMaterialLibrary))
    (:Finished
      (Rendering|Material|SetScalarParameterValue "/Game/SciFiGlitchPostPro/PostProcess/Material/postPrc.postPrc" (Utilities|String|StringToName (Utilities|String|Append "time" (Utilities|String|ToString(Integer) (Variables|Default|Getid)))) 0.0 :!class /Script/Engine.KismetMaterialLibrary)
      (Utilities|FlowControl|Delay 0.1)
      (Actor|DestroyActor))))

(event EventBeginPlay)

(event Collision|EventActorBeginOverlap
  (params (OtherActor :type Actor%20Object%20Reference)))

(event EventTick
  (params (DeltaSeconds :type Float%20%28single-precision%29)))

(fn ConstructionScript)