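; BP_Planet is a planet actor that orbits a referenced Sun actor.
; Each tick it rotates its offset from the Sun around an orbit axis at a rate set by Period, then points the material's Light Direction parameter at the Sun.
; The dynamic material setup for rotation, clouds and lighting is disconnected, and the construction script's GenerateOrbit branch does nothing.
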(event EventTick
  (params (DeltaSeconds :type Float%20%28single-precision%29))
  (Utilities|IsValid (Variables|Default|GetSun)
    (:Is%20Valid
      ;[1 1 1] orbit
      (bind _output_get (Variables|Default|SetOrbitDirection (- (Transformation|GetActorLocation) (Transformation|GetActorLocation (Variables|Default|GetSun)))))
      (Transformation|AddActorWorldOffset (- (Math|Vector|RotateVectorAroundAxis _output_get (/ (Utilities|Time|GetWorldDeltaSeconds) (/ (Variables|Default|GetPeriod) 3.6e+02)) (Variables|Default|GetOrbitAxsis)) (Variables|Default|GetOrbitDirection)))
      ;[1 1 1] set light direction
      (Rendering|Material|SetVectorParameterValue (Variables|Default|GetMaterialInstance) "Light Direction" (Math|Conversions|ToLinearColor(Vector) (Math|Vector|GetForwardVector (Math|Rotator|FindLookatRotation (Transformation|GetActorLocation) (Transformation|GetActorLocation (Variables|Default|GetSun))))) :!class /Script/Engine.MaterialInstanceDynamic))))

(fn ConstructionScript
  (if (Variables|Default|GetGenerateOrbit)
    (Utilities|IsValid (Variables|Default|GetSun))))