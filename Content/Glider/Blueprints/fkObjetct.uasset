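; Moving scenery actor for the Glider game: a randomized cluster of instanced meshes that rushes along +X and destroys itself once world X reaches 100.
; The construction script scatters instances within Radius in a flattened spread with random rotation and scale, and picks a mostly-forward velocity with slight jitter.
; Tick applies that velocity as an unswept local offset.
; Hit only prints a debug string, and the spin and actor-scale nodes are disconnected.
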(event EventBeginPlay)

(event Collision|EventActorBeginOverlap
  (params (OtherActor :type Actor%20Object%20Reference)))

(event EventTick
  (params (DeltaSeconds :type Float%20%28single-precision%29))
  (Transformation|AddActorLocalOffset (* (Variables|Default|Getdirection) DeltaSeconds) false false)
  (if (>= (.X (Math|Vector|BreakVector (Transformation|GetActorLocation))) 1e+02)
    (Actor|DestroyActor)))

(event Collision|EventHit
  (params (MyComp :type Primitive%20Component%20Object%20Reference) (Other :type Actor%20Object%20Reference) (OtherComp :type Primitive%20Component%20Object%20Reference) (bSelfMoved :type Boolean) (HitLocation :type Vector :default "0, 0, 0") (HitNormal :type Vector :default "0, 0, 0") (NormalImpulse :type Vector :default "0, 0, 0") (Hit :type Hit%20Result%20Structure%20%28by%20ref%29))
  (Development|PrintString "Hello"))

(fn ConstructionScript
  (bind _returnvalue (Math|Random|RandomFloatinRange 5.0 27.0))
  (Variables|Default|Setdirection (+ (* (Math|Random|RandomUnitVector) (Math|Random|RandomFloatinRange 1e+02 2.5e+02)) "14000.000000, 0, 0"))
  (Variables|Default|Setrotm (Math|Random|RandomRotator true))
  (for _index (range 0 20)
    (Components|InstancedStaticMesh|AddInstance (Variables|Default|GetInstancedStaticMesh) (Math|Transform|MakeTransform (* (Math|Vector|Normalize (Math|Vector|MakeVector (Math|Random|RandomFloatinRange -0.2 0.3) (Math|Random|RandomFloatinRange -1.0 1.0) (Math|Random|RandomFloatinRange -0.1 0.1))) (Math|Random|RandomFloatinRange 0.0 (Variables|Default|Getradius))) (Math|Random|RandomRotator false) (Math|Vector|MakeVector _returnvalue _returnvalue _returnvalue)))))