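; Planet actor that orbits on a spring arm and shades its mesh toward a Sun reference.
; Tick advances the angle by Period, sets arm length and yaw from CalculateElipseParams for an elliptical path, and leaves a randomly colored debug-point trail.
; The construction script builds the dynamic material with rotation and cloud speeds, and scales the mesh.
; Light direction updates only while Sun is valid; its parent-actor assignment is unwired.
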(event EventTick
  (params (DeltaSeconds :type Float%20%28single-precision%29))
  (bind _ecliptic (Variables|Default|GetEcliptic))
  (bind (_distancetofocus _aglerotationaroundfocus) (Utilities|CalculateElipseParams _ecliptic))
  (Variables|Default|SetcurrentAgle (select (> (+ (Variables|Default|GetcurrentAgle) (* (/ DeltaSeconds (Variables|Default|GetPeriod)) 3.6e+02)) 3.6e+02) (- (+ (Variables|Default|GetcurrentAgle) (* (/ DeltaSeconds (Variables|Default|GetPeriod)) 3.6e+02)) 3.6e+02) (+ (Variables|Default|GetcurrentAgle) (* (/ DeltaSeconds (Variables|Default|GetPeriod)) 3.6e+02))))
  (Variables|/Script/Engine.SpringArmComponent|SetTargetArmLength (Variables|Default|GetSpringArm) _distancetofocus)
  (Rendering|Debug|DrawDebugPoint (Transformation|GetWorldLocation (Variables|Default|GetStaticMesh)) 1.0 (Variables|Default|GetNewVar_0) (* (Variables|Default|GetPeriod) 2e+02))
  (Transformation|SetRelativeRotation (Variables|Default|GetSpringArm) (Math|Rotator|MakeRotator 0.0 0.0 _aglerotationaroundfocus) false false)
  (Utilities|IsValid (Variables|Default|GetSun)
    (:Is%20Valid
      ;[1 1 1] set light direction
      (Rendering|Material|SetVectorParameterValue (Variables|Default|GetPlanetMaterialInstance) "Light Direction" (Math|Conversions|ToLinearColor(Vector) (Math|Vector|GetForwardVector (Math|Rotator|FindLookatRotation (Transformation|GetWorldLocation (Variables|Default|GetStaticMesh)) (Transformation|GetActorLocation (Variables|Default|GetSun))))) :!class /Script/Engine.MaterialInstanceDynamic))))

(event EventBeginPlay)

(fn ConstructionScript
  (CallFunction|SetPlaet))

(fn SetPlaet
  (bind _sun (Variables|Default|GetSun))
  (bind _planetscale (Variables|Default|GetplanetScale))
  (Utilities|FlowControl|Sequence
    (:then_0
      (bind _returnvalue (Rendering|Material|CreateDynamicMaterialInstance (Variables|Default|GetStaticMesh) 0 "/Game/Glider/Materials/M_PlanetShader_Inst.M_PlanetShader_Inst" :!class /Script/Engine.PrimitiveComponent))
      (Variables|Default|SetPlanetMaterialInstance _returnvalue)
      (Rendering|Material|SetVectorParameterValue _returnvalue "Rotation Speed" (Math|Conversions|ToLinearColor(Vector) (Variables|Default|GetRotationSpeed)) :!class /Script/Engine.MaterialInstanceDynamic)
      (Rendering|Material|SetVectorParameterValue _returnvalue "Clouds Speed" (Math|Conversions|ToLinearColor(Vector) (Variables|Default|GetCloudsSpeed)) :!class /Script/Engine.MaterialInstanceDynamic)
      (Utilities|IsValid _sun
        (:Is%20Valid
          (Rendering|Material|SetVectorParameterValue _returnvalue "Light Direction" (Math|Conversions|ToLinearColor(Vector) (Math|Vector|GetForwardVector (Math|Rotator|FindLookatRotation (Transformation|GetWorldLocation (Variables|Default|GetStaticMesh)) (Transformation|GetActorLocation _sun)))) :!class /Script/Engine.MaterialInstanceDynamic))))
    (:then_1
      (Variables|/Script/Engine.SpringArmComponent|SetTargetArmLength (Variables|Default|GetSpringArm) (.distanceToFocus (Utilities|CalculateElipseParams (Variables|Default|GetEcliptic)))))
    (:then_2
      (Transformation|SetWorldScale3D (Variables|Default|GetStaticMesh) (Math|Vector|MakeVector _planetscale _planetscale _planetscale)))
    (:then_3
      (Variables|Default|SetNewVar_0 (Utilities|Struct|MakeLinearColor (Math|Random|RandomFloatinRange 0.0 1.0) (Math|Random|RandomFloatinRange 0.0 1.0) (Math|Random|RandomFloatinRange 0.0 1.0) 1.0)))))