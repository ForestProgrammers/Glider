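; Physics ball actor that can be punched across the level and breaks Wall actors it hits.
; The punch event applies a horizontal, mass-independent velocity impulse toward a given point, scaled by power.
; On hitting a wall component different from the last one recorded, it calls the wall's Destruct along the reversed hit normal impulse.
; It then spawns a Splasher at the impact, with power scaled by ball mass and speed.
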(event Custom|punch
  (params (dir :type Vector) (power :type Float%20%28single-precision%29))
  (bind _returnvalue (Transformation|GetActorLocation))
  (bind _returnvalue_2 (- dir _returnvalue))
  (bind (_x _y) (Math|Vector|BreakVector _returnvalue_2))
  (Physics|AddImpulse (Variables|Default|GetSphere) (* (Math|Vector|Normalize (Math|Vector|MakeVector _x _y 0.0)) (* power 1e+03)) "None" true))

(event EventBeginPlay)

(event Collision|EventActorBeginOverlap
  (params (OtherActor :type Actor%20Object%20Reference)))

(event EventTick
  (params (DeltaSeconds :type Float%20%28single-precision%29)))

(event Collision|EventHit
  (params (MyComp :type Primitive%20Component%20Object%20Reference) (Other :type Actor%20Object%20Reference) (OtherComp :type Primitive%20Component%20Object%20Reference) (bSelfMoved :type Boolean) (HitLocation :type Vector :default "0, 0, 0") (HitNormal :type Vector :default "0, 0, 0") (NormalImpulse :type Vector :default "0, 0, 0") (Hit :type Hit%20Result%20Structure%20%28by%20ref%29))
  (bind _sphere (Variables|Default|GetSphere))
  (if (== (Utilities|GetClass Other) "/Game/Glider/Blueprints/wall.wall_C")
    (if (not (== OtherComp (Variables|Default|GetlasrComp)))
      (bind _aswall (Utilities|Casting|CastTowall Other))
      (bind _returnvalue (Physics|GetPhysicsLinearVelocity _sphere "None"))
      (Default|Destruct _aswall 1.0 (* NormalImpulse -1.0))
      (Variables|Default|SetlasrComp OtherComp)
      (bind _returnvalue_2 (Game|SpawnActorfromClass "/Game/Glider/Blueprints/splasher.splasher_C" (Math|Transform|MakeTransform "0, 0, 0") "Undefined" 0 0))
      (Default|Splash _returnvalue_2 HitLocation (* (* (Physics|GetMass _sphere) (/ (Math|Vector|VectorLength _returnvalue) 1e+04)) 1e+02)))))

(fn ConstructionScript)